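; Tree actor for an apple-dropping game that slides along X, randomly reversing and spawning apples at its position.
; Tick applies a per-frame offset, not scaled by delta time, flips direction beyond the X bounds and destroys the tree at or below zero height.
; Looping timers are set alongside random-chance functions for apple spawning with sound and direction changes.
; Speed and reversal probability come from AppleGameState.
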(event `self.ReceiveBeginPlay`
  (`|ExecutionSequence`
    (:`then_0`
      (bind _asapple_game_state (cast `/Game/Blueprints/AppleGameState` (`GameplayStatics.GetGameState`)))
      (set `self.AppleGameState` _asapple_game_state))
    (:`then_1`
      (set `self.TreeTransformVector` (`KismetMathLibrary.MakeVector` (`/Game/Blueprints/AppleGameState.TreeSpeed` (`self.AppleGameState`)))))
    (:`then_2`
      (`KismetSystemLibrary.K2_SetTimerDelegate` (`|CreateDelegate` :!event `ChangeDirectionCallback`) 1.0 true))
    (:`then_3`
      (`KismetSystemLibrary.K2_SetTimerDelegate` (`|CreateDelegate` :!event `SpawnAnApple`) 0.2 true))))

(event `self.ReceiveActorBeginOverlap`
  (params (OtherActor :type "Actor Object Reference")))

(event `self.ReceiveTick`
  (params (DeltaSeconds :type "Float (single-precision)"))
  (`self.K2_AddActorWorldOffset` (`self.TreeTransformVector`))
  (if (<= (.z (`self.K2_GetActorLocation`)) 0.0)
    (`self.K2_DestroyActor`)
    (elif (> (`KismetMathLibrary.Abs` (`KismetMathLibrary.BreakVector3f` (`self.K2_GetActorLocation`))) 1500.0)
      (`self.ChangeDirection`))))

(fn `ChangeDirection`
  (if (> (.x (`self.TreeTransformVector`)) 0.0)
    (set `self.TreeTransformVector` (`KismetMathLibrary.MakeVector` (* (`/Game/Blueprints/AppleGameState.TreeSpeed` (`self.AppleGameState`)) -1.0)))
    (else
      (set `self.TreeTransformVector` (`KismetMathLibrary.MakeVector` (`/Game/Blueprints/AppleGameState.TreeSpeed` (`self.AppleGameState`)))))))

(fn `ChangeDirectionCallback`
  (if (< (`KismetMathLibrary.RandomIntegerInRange` 0 100) (`/Game/Blueprints/AppleGameState.TreeDirectionChangeProbability` (`self.AppleGameState`)))
    (`self.ChangeDirection`)))

(fn `SpawnAnApple`
  (switch `int` (`KismetMathLibrary.RandomIntegerInRange` 0 4)
    (:`0`
      (`|SpawnActorFromClass` "/Game/Blueprints/AppleActorBP.AppleActorBP_C" (`self.GetTransform`) "AlwaysSpawn" "OverrideRootScale" null null)
      (`GameplayStatics.PlaySoundAtLocation` "/Game/Pictures/apple_spawned.apple_spawned" (0.0 0.0 0.0) (struct) 1.0 1.0 0.0 null null null null))))

(fn `UserConstructionScript`)