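; Player basket pawn for an apple-catching game that follows the mouse horizontally and collects apples on overlap.
; Each tick it maps clamped cursor X to the game state's ortho camera width, stopping once DiedState is set.
; Overlapped apples are always destroyed, but only count through AppleGameState and play a sound while alive.
; BeginPlay caches that game state and resets its counter; R reloads MainLevel.
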(event `self.ReceiveBeginPlay`
  (set `self.bGenerateOverlapEventsDuringLevelStreaming` true)
  (bind _asapple_game_state (cast `/Game/Blueprints/AppleGameState` (`GameplayStatics.GetGameState`)))
  (bind _output_get (set `self.GameState` _asapple_game_state))
  (`/Game/Blueprints/AppleGameState.ResetApplesCounter` _output_get))

(event `self.ReceiveActorBeginOverlap`
  (params (OtherActor :type "Actor Object Reference"))
  (bind _asapple_actor_bp (cast `/Game/Blueprints/AppleActorBP` OtherActor))
  (`self.K2_DestroyActor` _asapple_actor_bp)
  (if (not (`/Game/Blueprints/AppleGameState.DiedState` (`self.GameState`)))
    (`/Game/Blueprints/AppleGameState.AppleCollected` (`self.GameState`))
    (`GameplayStatics.PlaySoundAtLocation` "/Game/Pictures/apple_eaten.apple_eaten" (0.0 0.0 0.0) (struct) 1.0 1.0 0.0 null null null null)))

(event `Key|R`
  (params (Key :type "Key Structure"))
  (:`Pressed`
    (`GameplayStatics.OpenLevel` "MainLevel")))

(event `self.ReceiveTick`
  (params (DeltaSeconds :type "Float (single-precision)"))
  (bind _x (`KismetMathLibrary.BreakVector2D` (`WidgetLayoutLibrary.GetViewportSize`)))
  (bind (_x_2 _y _z) (`KismetMathLibrary.BreakVector3f` (`self.K2_GetActorLocation`)))
  (if (not (`/Game/Blueprints/AppleGameState.DiedState` (`self.GameState`)))
    (bind _returnvalue (`WidgetLayoutLibrary.GetMousePositionOnViewport`))
    (`self.K2_SetActorLocation` (`KismetMathLibrary.MakeVector` (- (* (/ (`/Game/Blueprints/AppleGameState.OrthoWidth` (`self.GameState`)) _x) (`KismetMathLibrary.FMax` (`KismetMathLibrary.FMin` (`KismetMathLibrary.BreakVector2D` _returnvalue) _x) 0.0)) (/ (`/Game/Blueprints/AppleGameState.OrthoWidth` (`self.GameState`)) 2.0)) _y _z))))

(fn `UserConstructionScript`)