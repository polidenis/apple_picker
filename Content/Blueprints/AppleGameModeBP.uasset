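; Game mode for an apple-catching style game that sets up the basket, camera and tree on BeginPlay.
; It caches AppleGameState, then spawns a basket pawn and an orthographic, fixed-aspect camera sized from that state and set as view target.
; The tree spawns high above the player pawn.
; The new basket's assignment to Basket is disconnected, so possession and the return value use a variable this graph never fills.
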(event `self.ReceiveBeginPlay`
  (`|ExecutionSequence`
    (:`then_0`
      (`self.EnableInput` (`GameplayStatics.GetPlayerController` 0) null)
      (bind _asapple_game_state (cast `/Game/Blueprints/AppleGameState` (`GameplayStatics.GetGameState`)))
      (set `self.AppleGameState` _asapple_game_state))
    (:`then_1`
      (bind _returnvalue (`self.SpawnBacketPawn`))
      (set `self.Basket` _returnvalue))
    (:`then_2`
      (bind _returnvalue_2 (`self.SpawnTreeActor`))
      (set `self.Tree` _returnvalue_2))))

(fn `SpawnBacketPawn`
  (returns (ReturnValue :type "/Game/Blueprints/BasketPawnBP Object Reference"))
  (locals (ActorsCamera :type "CameraComponent Object Reference") (Basket :type "/Game/Blueprints/BasketPawnBP Object Reference"))
  (bind _returnvalue (`|SpawnActorFromClass` "/Game/Blueprints/BasketPawnBP.BasketPawnBP_C" (`KismetMathLibrary.MakeTransform` (0.0 0.0 67.0)) "AlwaysSpawn" "OverrideRootScale" null null))
  (`Controller.Possess` (`GameplayStatics.GetPlayerController` 0) (`local.Basket`))
  (bind _returnvalue_2 (`|SpawnActorFromClass` "/Script/Engine.CameraActor" (`KismetMathLibrary.MakeTransform` (0.0 2000.0 900.0) (struct :`Yaw` 270.0)) "AlwaysSpawn" "OverrideRootScale" null null))
  (`|ExecutionSequence`
    (:`then_0`
      (set `local.ActorsCamera` (`CameraActor.CameraComponent` _returnvalue_2)))
    (:`then_1`
      (`CameraComponent.SetProjectionMode` (`local.ActorsCamera`) "Orthographic"))
    (:`then_2`
      (`CameraComponent.SetConstraintAspectRatio` (`local.ActorsCamera`) true))
    (:`then_3`
      (`CameraComponent.SetOrthoWidth` (`local.ActorsCamera`) (`/Game/Blueprints/AppleGameState.OrthoWidth` (`self.AppleGameState`))))
    (:`then_4`
      (`PlayerController.SetViewTargetWithBlend` (`GameplayStatics.GetPlayerController` 0) _returnvalue_2 0.0 "VTBlend_Linear" 0.0 false))
    (:`then_5`
      (return (`local.Basket`)))))

(fn `SpawnTreeActor`
  (returns (ReturnValue :type "/Game/Blueprints/TreeActorBP Object Reference"))
  (bind _returnvalue (`|SpawnActorFromClass` "/Game/Blueprints/TreeActorBP.TreeActorBP_C" (`KismetMathLibrary.Conv_VectorToTransform` (+ (`self.K2_GetActorLocation` (`GameplayStatics.GetPlayerPawn` 0)) (0.0 0.0 1500.0))) "AlwaysSpawn" "OverrideRootScale" null null))
  (return _returnvalue))

(fn `UserConstructionScript`)