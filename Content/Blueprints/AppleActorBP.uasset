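; Falling apple actor that ends the player's run when it reaches the ground, by setting the died state on AppleGameState.
; The construction script caches the game state and picks a random speed within its lower and upper bounds.
; Tick offsets the actor along Z by that speed without delta-time scaling, then destroys it once Z is zero or below.
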(event `self.ReceiveBeginPlay`)

(event `self.ReceiveTick`
  (params (DeltaSeconds :type "Float (single-precision)"))
  (`self.K2_AddActorWorldOffset` (`KismetMathLibrary.MakeVector` 0.0 0.0 (`self.AppleSpeed`)))
  (if (<= (.z (`self.K2_GetActorLocation`)) 0.0)
    (`self.K2_DestroyActor`)
    (`/Game/Blueprints/AppleGameState.SetDiedState` (`self.AppleGameState`) true)))

(fn `UserConstructionScript`
  (bind _applegamestate (`self.AppleGameState`))
  (bind _asapple_game_state (cast `/Game/Blueprints/AppleGameState` (`GameplayStatics.GetGameState`)))
  (set `self.AppleGameState` _asapple_game_state)
  (set `self.AppleSpeed` (`KismetMathLibrary.RandomFloatInRange` (`/Game/Blueprints/AppleGameState.AppleSpeedLower` _applegamestate) (`/Game/Blueprints/AppleGameState.AppleSpeedHigher` _applegamestate))))