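; AppleGameState is the game state for an apple-collecting game, holding tuning values, the collected count and the died state.
; BeginPlay sets camera ortho width, tree speed, apple speed bounds and tree direction-change probability.
; Functions increment or reset the count and set the died state, broadcasting changes through event dispatchers.
; One second after BeginPlay, it also broadcasts hard-coded test log entries through a log event dispatcher.
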(event `self.ReceiveBeginPlay`
  (`|ExecutionSequence`
    (:`then_0`
      (set `self.OrthoWidth` 3000.0))
    (:`then_1`
      (set `self.TreeSpeed` 3.0))
    (:`then_2`
      (set `self.AppleSpeedLower` -1.0))
    (:`then_3`
      (set `self.AppleSpeedHigher` -4.0))
    (:`then_4`
      (set `self.TreeDirectionChangeProbability` 15))
    (:`then_5`
      (`KismetSystemLibrary.Delay` 1.0)
      (`self.Add Test Logs`))))

(fn `Add Test Logs`
  (`self.LogEventDispatcher` (make `/Game/Data/SLogData` "/Game/Pictures/w1.w1" "B" "24" true))
  (`self.LogEventDispatcher` (make `/Game/Data/SLogData` "/Game/Pictures/w1.w1" "D" "sdfsd24"))
  (`self.LogEventDispatcher` (make `/Game/Data/SLogData` "/Game/Pictures/w2.w2" "C" "2dff4" true))
  (`self.LogEventDispatcher` (make `/Game/Data/SLogData` "/Game/Pictures/w3.w3" "AE" "Sdfge"))
  (`self.LogEventDispatcher` (make `/Game/Data/SLogData` "/Game/Pictures/w2.w2" "FA" "Sdfge")))

(fn `AppleCollected`
  (bind _result (`/Engine/EditorBlueprintResources/StandardMacros.IncrementInt` (`self.ApplesCollectedCount`))
    (:`  `
      (bind _output_get (set `self.ApplesCollectedCount` _result))
      (`self.ScoreChangedDispatcher` _output_get))))

(fn `ResetApplesCounter`
  (bind _output_get (set `self.ApplesCollectedCount` 0))
  (`self.ScoreChangedDispatcher` _output_get))

(fn `SetDiedState`
  (params (State :type Boolean))
  (bind _output_get (set `self.DiedState` State))
  (`self.DiedStateChangedDispatcher` _output_get))

(fn `UserConstructionScript`)